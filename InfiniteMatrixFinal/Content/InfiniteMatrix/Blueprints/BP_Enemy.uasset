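; BP_Enemy is a short-lived enemy that damages the player on contact and can be shot for score.
; Player overlap lowers health and, at zero, shows restart and resets health, score and forward speed.
; Projectile overlap destroys the enemy; the end-overlap event then removes the projectile and awards a point.
; It writes directly to BP_Player's stats and widgets, raising forward speed every tenth point up to a cap.
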(event OnComponentBeginOverlap(BadGuy)
  (params (OverlappedComponent :type Primitive%20Component%20Object%20Reference) (OtherActor :type Actor%20Object%20Reference) (OtherComp :type Primitive%20Component%20Object%20Reference) (OtherBodyIndex :type Integer) (bFromSweep :type Boolean) (SweepResult :type Hit%20Result%20Structure%20%28by%20ref%29))
  (bind _asbp_player (Utilities|Casting|CastToBP_Player OtherActor)
    (:then
      (bind _output_get (Variables|/Game/InfiniteMatrix/Blueprints/BP_Player.BP_Player_C|SetHealth _asbp_player (- (Variables|/Game/InfiniteMatrix/Blueprints/BP_Player.BP_Player_C|GetHealth _asbp_player) 1)))
      (Default|UpdateHealthBar (Variables|/Game/InfiniteMatrix/Blueprints/BP_Player.BP_Player_C|GetHealthBar _asbp_player) (Math|Conversions|ToFloat(Integer) _output_get))
      (bind _output_get_2 (Variables|/Game/InfiniteMatrix/Blueprints/BP_Player.BP_Player_C|SetIsDead _asbp_player (<= _output_get 0)))
      (if _output_get_2
        (Default|DisplayRestart _asbp_player)
        (bind _output_get_3 (Variables|/Game/InfiniteMatrix/Blueprints/BP_Player.BP_Player_C|SetHealth _asbp_player 10))
        (Default|UpdateHealthBar (Variables|/Game/InfiniteMatrix/Blueprints/BP_Player.BP_Player_C|GetHealthBar _asbp_player) (Math|Conversions|ToFloat(Integer) _output_get_3))
        (bind _output_get_4 (Variables|/Game/InfiniteMatrix/Blueprints/BP_Player.BP_Player_C|SetScore _asbp_player 0))
        (Default|UpdateScore (Variables|/Game/InfiniteMatrix/Blueprints/BP_Player.BP_Player_C|GetScoreCnt _asbp_player) _output_get_4)
        (Variables|/Game/InfiniteMatrix/Blueprints/BP_Player.BP_Player_C|SetForwardSpeed _asbp_player 2e+03)))
    (:CastFailed
      (Utilities|Casting|CastToBP_Projectile OtherActor)
      (Actor|DestroyActor))))

(event OnComponentEndOverlap(BadGuy)
  (params (OverlappedComponent :type Primitive%20Component%20Object%20Reference) (OtherActor :type Actor%20Object%20Reference) (OtherComp :type Primitive%20Component%20Object%20Reference) (OtherBodyIndex :type Integer))
  (bind _asbp_projectile (Utilities|Casting|CastToBP_Projectile OtherActor))
  (Actor|DestroyActor _asbp_projectile)
  (bind _asbp_player (Utilities|Casting|CastToBP_Player (Game|Player|GetPlayerPawn 0)))
  (bind _output_get (Variables|/Game/InfiniteMatrix/Blueprints/BP_Player.BP_Player_C|SetScore _asbp_player (+ (Variables|/Game/InfiniteMatrix/Blueprints/BP_Player.BP_Player_C|GetScore _asbp_player) 1)))
  (Default|UpdateScore (Variables|/Game/InfiniteMatrix/Blueprints/BP_Player.BP_Player_C|GetScoreCnt _asbp_player) _output_get)
  (if (== (Math|Integer|%(Integer) _output_get 10) 0)
    (if (not (>= (+ (Variables|/Game/InfiniteMatrix/Blueprints/BP_Player.BP_Player_C|GetForwardSpeed _asbp_player) 1e+02) 4e+03))
      (Variables|/Game/InfiniteMatrix/Blueprints/BP_Player.BP_Player_C|SetForwardSpeed _asbp_player (+ (Variables|/Game/InfiniteMatrix/Blueprints/BP_Player.BP_Player_C|GetForwardSpeed _asbp_player) 1e+02)))))

(event EventBeginPlay
  (Actor|SetLifeSpan 1e+01))

(event Collision|EventActorBeginOverlap
  (params (OtherActor :type Actor%20Object%20Reference)))

(event EventTick
  (params (DeltaSeconds :type Float%20%28single-precision%29)))

(fn ConstructionScript)